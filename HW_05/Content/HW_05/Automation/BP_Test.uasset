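; Automation functional test that grades the BP_Exercise damage formula and the level's tagged instances of it.
; PrepareTest requires two "Enemy" actors and one "Boss", then spawns a default BP_Exercise as the baseline target.
; StartTest calls CalculateDamage with fixed inputs, asserting in turn the default result, the enemies' summed damage and the boss damage.
; The first failed assertion fails the test, while bad setup or an invalid target reports Invalid.
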(event `self.ReceivePrepareTest`
  (bind _outactors (`GameplayStatics.GetAllActorsOfClassWithTag` "/Game/HW_05/Blueprints/BP_Exercise.BP_Exercise_C" "Enemy"))
  (set `self.Enemies` _outactors)
  (bind _outactors_2 (`GameplayStatics.GetAllActorsOfClassWithTag` "/Game/HW_05/Blueprints/BP_Exercise.BP_Exercise_C" "Boss"))
  (set `self.Bosses` _outactors_2)
  (if (and (== (`KismetArrayLibrary.Array_Length` (`self.Enemies`)) 2) (== (`KismetArrayLibrary.Array_Length` (`self.Bosses`)) 1))
    (bind _returnvalue (`|SpawnActorFromClass` "/Game/HW_05/Blueprints/BP_Exercise.BP_Exercise_C" (`KismetMathLibrary.MakeTransform` (0.0 0.0 0.0)) "Undefined" "OverrideRootScale" null null))
    (bind _output_get (set `self.Target` _returnvalue))
    (`/Engine/EditorBlueprintResources/StandardMacros.IsValid` _output_get
      (:`Is Valid`
        (set `self.TestReady` true))
      (:`Is Not Valid`
        (`self.FinishTest` "Invalid" "Failed to spawn default BP_Exercise!")))
    (else
      (`self.FinishTest` "Invalid" "Error in user BP_Exercise instances setup!"))))

(event `self.ReceiveStartTest`
  (bind _target (`self.Target`)
    (:`then`
      (bind _result (`/Game/HW_05/Blueprints/BP_Exercise.CalculateDamage` _target 100.0 1.0))
      (bind _returnvalue (`self.AssertEqual_Float` _result 3000.0 "Test user formula using default values."))
      (if _returnvalue
        (for _array_element (`self.Enemies`)
          (bind _result_2 (`/Game/HW_05/Blueprints/BP_Exercise.CalculateDamage` _array_element 100.0 1.0))
          (set `self.EnemyDamageBuffer` (+ (`self.EnemyDamageBuffer`) _result_2)))
        (bind _returnvalue_2 (`self.AssertEqual_Float` (`self.EnemyDamageBuffer`) 3000.0 "Test summary enemies damage"))
        (if _returnvalue_2
          (bind _result_3 (`/Game/HW_05/Blueprints/BP_Exercise.CalculateDamage` (`|GetArrayItem` (`self.Bosses`)) 100.0 1.0))
          (bind _returnvalue_3 (`self.AssertEqual_Float` _result_3 10000.0 "Test boss damage"))
          (if _returnvalue_3
            (`self.FinishTest` "Succeeded" "Congrats!")
            (else
              (`self.FinishTest` "Failed" "Boss damage assertion failed!")))
          (else
            (`self.FinishTest` "Failed" "Enemy damage assertion failed!")))
        (else
          (`self.FinishTest` "Failed" "Default setup damage assertion failed!"))))
    (:`else`
      (`self.FinishTest` "Invalid" "Target is not valid!"))))

(fn `UserConstructionScript`)