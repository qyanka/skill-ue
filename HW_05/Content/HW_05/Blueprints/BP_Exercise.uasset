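; BP_Exercise is a homework Blueprint that computes attack damage from weapon damage, speed, base damage and hit count.
; CalculateDamage branches on IsCritical into the OnCritical or OnUncritical subgraph.
; Both add weapon damage to speed-scaled base damage and multiply by Hits, with criticals doubled.
; The result is stored in the Damage variable, while the function itself always returns zero.
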(fn `CalculateDamage`
  (params (WeaponDamage :type "Float (double-precision)") (Speed :type "Float (double-precision)"))
  (returns (Result :type "Float (double-precision)"))
  (locals (Damage :type "Float (double-precision)"))
  (if (`self.IsCritical`)
    (`self.OnCritical` WeaponDamage Speed)
    (else
      (`self.OnUncritical` WeaponDamage Speed)))
  (return 0.0))

(fn `UserConstructionScript`)