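; BP_Char is a player character Blueprint that handles movement, look, jump and sprint through Enhanced Input.
; BeginPlay adds the IMC_Char mapping context to player controller 0's input subsystem.
; Input actions drive movement along the actor's forward and right vectors, feed controller pitch and yaw, and start or stop jumping.
; Sprint raises the movement component's max walk speed while held and lowers it on completion.
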(event `self.ReceiveBeginPlay`
  (`EnhancedInputSubsystemInterface.AddMappingContext` (pcsubsystem `EnhancedInputLocalPlayerSubsystem` (`GameplayStatics.GetPlayerController` 0)) "/Game/Test/Characters/Char/Input/IMC_Char.IMC_Char" 0 (struct)))

(event `EnhancedInput|/Game/Test/Characters/Char/Input/Actions/IA_CharMove`
  (params (ActionValue :type "Vector2D Structure") (ElapsedSeconds :type "Float (double-precision)") (TriggeredSeconds :type "Float (double-precision)") (InputAction :type "InputAction Object Reference" :default "/Game/Test/Characters/Char/Input/Actions/IA_CharMove.IA_CharMove"))
  (:`Triggered`
    (`self.AddMovementInput` (`self.GetActorForwardVector`) ActionValue_Y)
    (`self.AddMovementInput` (`self.GetActorRightVector`) ActionValue_X)))

(event `EnhancedInput|/Game/Test/Characters/Char/Input/Actions/IA_CharLook`
  (params (ActionValue :type "Vector2D Structure") (ElapsedSeconds :type "Float (double-precision)") (TriggeredSeconds :type "Float (double-precision)") (InputAction :type "InputAction Object Reference" :default "/Game/Test/Characters/Char/Input/Actions/IA_CharLook.IA_CharLook"))
  (:`Triggered`
    (`self.AddControllerPitchInput` ActionValue_Y)
    (`self.AddControllerYawInput` ActionValue_X)))

(event `EnhancedInput|/Game/Test/Characters/Char/Input/Actions/IA_CharJump`
  (params (ActionValue :type Boolean) (ElapsedSeconds :type "Float (double-precision)") (TriggeredSeconds :type "Float (double-precision)") (InputAction :type "InputAction Object Reference" :default "/Game/Test/Characters/Char/Input/Actions/IA_CharJump.IA_CharJump"))
  (:`Triggered`
    (`self.Jump`))
  (:`Completed`
    (`self.StopJumping`)))

(event `EnhancedInput|/Game/Test/Characters/Char/Input/Actions/IA_CharSprint`
  (params (ActionValue :type Boolean) (ElapsedSeconds :type "Float (double-precision)") (TriggeredSeconds :type "Float (double-precision)") (InputAction :type "InputAction Object Reference" :default "/Game/Test/Characters/Char/Input/Actions/IA_CharSprint.IA_CharSprint"))
  (bind _charactermovement (`self.CharacterMovement`))
  (:`Triggered`
    (set `CharacterMovementComponent.MaxWalkSpeed` 1500.0 _charactermovement))
  (:`Completed`
    (set `CharacterMovementComponent.MaxWalkSpeed` 600.0 _charactermovement)))

(fn `UserConstructionScript`)