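; BP_Platrol is a patrolling actor that moves back and forth and damages whatever it hits.
; Each Tick it moves along Direction at Speed without sweep, then line-traces one step ahead on the Visibility channel.
; A blocking trace flips Direction on X and zeroes Y and Z, so patrol continues only along X.
; Hit events apply fixed damage to the other actor after a short delay.
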(event `self.ReceiveTick`
  (params (DeltaSeconds :type "Float (single-precision)"))
  (bind _vectorlocation (`self.VectorMoveForward` DeltaSeconds (`self.Direction`) (`self.Speed`)))
  (`self.ReverseIfHitted` _vectorlocation))

(event `self.ReceiveHit`
  (params (MyComp :type "PrimitiveComponent Object Reference") (Other :type "Actor Object Reference") (OtherComp :type "PrimitiveComponent Object Reference") (bSelfMoved :type Boolean) (HitLocation :type "Vector Structure") (HitNormal :type "Vector Structure") (NormalImpulse :type "Vector Structure") (Hit :type "HitResult Structure (by ref)"))
  (`KismetSystemLibrary.Delay` 0.2)
  (`GameplayStatics.ApplyDamage` Other 50.0 null self))

(fn `ReverseIfHitted`
  (params (VectorLocation :type "Vector Structure"))
  (bind (_outhit _returnvalue) (`KismetSystemLibrary.LineTraceSingle` (`self.K2_GetActorLocation`) VectorLocation "TraceTypeQuery1"))
  (if _returnvalue
    (set `self.Direction` (* (`self.Direction`) (-1.0 0.0 0.0)))))

(fn `UserConstructionScript`)

(fn `VectorMoveForward`
  (params (DeltaSeconds :type "Float (double-precision)") (Direction :type "Vector Structure") (Speed :type "Float (double-precision)"))
  (returns (VectorLocation :type "Vector Structure"))
  (bind _returnvalue (+ (`self.K2_GetActorLocation`) (* DeltaSeconds (* Speed Direction))))
  (`self.K2_SetActorLocation` _returnvalue)
  (return _returnvalue))