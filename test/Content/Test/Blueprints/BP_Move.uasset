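; BP_Move is a test Blueprint for moving an actor along X against its Direction, scaled by Speed and frame time.
; Each Tick draws a forward Visibility multi-line trace over that frame's travel distance, but its hit check is unused.
; A FlipFlop gates the swept offset on its A output behind a negated IsA check, so the move appears never to run.
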(event `self.ReceiveTick`
  (params (DeltaSeconds :type "Float (single-precision)"))
  (bind _returnvalue (`self.K2_GetActorLocation`))
  (bind _outhits (`KismetSystemLibrary.LineTraceMulti` :`Start` _returnvalue :`End` (+ _returnvalue (* (* (`self.GetActorForwardVector`) (`self.Speed`)) DeltaSeconds)) :`TraceChannel` "TraceTypeQuery1" :`DrawDebugType` "ForOneFrame"))
  (bind _isa (`/Engine/EditorBlueprintResources/StandardMacros.FlipFlop`)
    (:`A`
      (if (not _isa)
        (`self.K2_AddActorWorldOffset` (* (* (`self.Direction`) (-1.0 0.0 0.0)) (* DeltaSeconds (`self.Speed`))) true)))))

(fn `UserConstructionScript`)