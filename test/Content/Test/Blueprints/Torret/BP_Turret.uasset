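; BP_Turret is a test turret actor that checks for the first-person player character.
; Each tick it calls PlayerSearch and prints the boolean result; it has no aiming or firing logic.
; PlayerSearch runs a debug-drawn sphere trace from the Scene component and returns true if the hit actor casts to BP_FirstPersonCharacter.
; The trace end is the forward vector times SearchDistance, without the start location added.
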(event `self.ReceiveTick`
  (params (DeltaSeconds :type "Float (single-precision)"))
  (bind _isplayerfind (`self.PlayerSearch`))
  (`KismetSystemLibrary.PrintString` (`KismetStringLibrary.Conv_BoolToString` _isplayerfind)))

(fn `PlayerSearch`
  (returns (IsPlayerFind :type Boolean))
  (bind _scene (`self.Scene`))
  (bind (_outhit _returnvalue) (`KismetSystemLibrary.SphereTraceSingle` :`Start` (`SceneComponent.K2_GetComponentLocation` _scene) :`End` (* (`SceneComponent.GetForwardVector` _scene) (`self.SearchDistance`)) :`Radius` 30.0 :`TraceChannel` "TraceTypeQuery3" :`DrawDebugType` "ForOneFrame"))
  (if _returnvalue
    (cast `/Game/FirstPerson/Blueprints/BP_FirstPersonCharacter` (`.HitActor` (`GameplayStatics.BreakHitResult` _outhit))
      (:`then`
        (return true))
      (:`CastFailed`
        (return false)))
    (else
      (return false))))

(fn `UserConstructionScript`)