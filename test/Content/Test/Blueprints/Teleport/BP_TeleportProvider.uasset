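; Teleport pad that sends the first-person character to one of its TeleportTargets when they touch the Cube with Energy above zero.
; Each use advances a counter to cycle through the targets in order and drains the character's energy, with a DoOnce and short delay preventing immediate retriggering.
; A separate Box overlap tints the Cube orange while the character is inside and black otherwise, through a dynamic material instance.
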(event `self.ReceiveBeginPlay`
  (`self.ChangeColor` false))

(event `self.Box.OnComponentBeginOverlap`
  (params (OverlappedComponent :type "PrimitiveComponent Object Reference") (OtherActor :type "Actor Object Reference") (OtherComp :type "PrimitiveComponent Object Reference") (OtherBodyIndex :type Integer) (bFromSweep :type Boolean) (SweepResult :type "HitResult Structure (by ref)"))
  (cast `/Game/FirstPerson/Blueprints/BP_FirstPersonCharacter` OtherActor)
  (`self.ChangeColor` true))

(event `self.Box.OnComponentEndOverlap`
  (params (OverlappedComponent :type "PrimitiveComponent Object Reference") (OtherActor :type "Actor Object Reference") (OtherComp :type "PrimitiveComponent Object Reference") (OtherBodyIndex :type Integer))
  (cast `/Game/FirstPerson/Blueprints/BP_FirstPersonCharacter` OtherActor)
  (`self.ChangeColor` false))

(event `self.Cube.OnComponentBeginOverlap`
  (params (OverlappedComponent :type "PrimitiveComponent Object Reference") (OtherActor :type "Actor Object Reference") (OtherComp :type "PrimitiveComponent Object Reference") (OtherBodyIndex :type Integer) (bFromSweep :type Boolean) (SweepResult :type "HitResult Structure (by ref)"))
  (bind _asbp_first_person_character (cast `/Game/FirstPerson/Blueprints/BP_FirstPersonCharacter` OtherActor))
  (bind _output_get (set `self.As BP First Person Character` _asbp_first_person_character))
  (if (> (`/Game/FirstPerson/Blueprints/BP_FirstPersonCharacter.Energy` _output_get) 0.0)
    (`/Engine/EditorBlueprintResources/StandardMacros.DoOnce` false :!label _label
      (:`Completed`
        (`/Game/Test/Blueprints/Teleport/BP_TeleportTarget.Teleport` (`|GetArrayItem` (`self.TeleportTargets`) (mod (`self.TPCounter`) (`KismetArrayLibrary.Array_Length` (`self.TeleportTargets`)))) _output_get)
        (bind _result (`/Engine/EditorBlueprintResources/StandardMacros.IncrementInt` (`self.TPCounter`))
          (:`  `
            (set `self.TPCounter` _result)
            (`/Game/FirstPerson/Blueprints/BP_FirstPersonCharacter.ChangeEnergy` (`self.As BP First Person Character`) -100.0)
            (`KismetSystemLibrary.Delay` 0.1)
            (goto _label :!via `Reset`)))))))

(fn `ChangeColor`
  (params (IsReady :type Boolean))
  (bind _returnvalue (`PrimitiveComponent.CreateDynamicMaterialInstance` (`self.Cube`) 0 null "None"))
  (if IsReady
    (`MaterialInstanceDynamic.SetVectorParameterValue` _returnvalue "Color" (struct :`R` 1.0 :`G` 0.463416 :`B` 0.302706 :`A` 1.0))
    (else
      (`MaterialInstanceDynamic.SetVectorParameterValue` _returnvalue "Color" (struct :`A` 1.0)))))

(fn `UserConstructionScript`)