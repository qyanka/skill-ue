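; BP_Test is an automated functional test that checks whether a Target actor's TextRender component has been customized.
; On StartTest it reports Invalid when Target is not valid.
; It then fails if the text still matches DefaultText or the component's relative scale is exactly one on all axes, and succeeds otherwise, with a message for each outcome.
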(event `self.ReceiveStartTest`
  (bind _target (`self.Target`)
    (:`then`
      (bind _textrender (`/Game/HW_04/Blueprints/BP_Exercise.TextRender` _target))
      (if (`KismetTextLibrary.EqualEqual_TextText` (`TextRenderComponent.Text` _textrender) (`self.DefaultText`))
        (`self.FinishTest` "Failed" "Text is default!")
        (elif (== (`SceneComponent.RelativeScale3D` _textrender) (1.0 1.0 1.0))
          (`self.FinishTest` "Failed" "Text has default scale!")
          (else
            (`self.FinishTest` "Succeeded" "Congrats!")))))
    (:`else`
      (`self.FinishTest` "Invalid" "Target is not valid!"))))

(fn `UserConstructionScript`)