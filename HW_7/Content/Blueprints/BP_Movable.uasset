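; BP_Movable is an actor that wanders within a rectangular XY boundary by moving forward at Speed every tick.
; When it is outside the bounds and not facing their center, it turns to a random yaw.
; A DoOnce limits this to one turn until the actor is back inside, so the new heading is not guaranteed to lead back in.
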(event EventBeginPlay)

(event EventTick
  (params (DeltaSeconds :type Float%20%28single-precision%29))
  (Utilities|FlowControl|Sequence
    (:then_0
      (if (CallFunction|IsActorinBoundaries2D (Variables|Default|GetMin%20X) (Variables|Default|GetMax%20X) (Variables|Default|GetMin%20Y) (Variables|Default|GetMax%20Y))
        (goto _label Reset)
        (elif (<= (Math|Vector|DotProduct (Math|Vector|Normalize (- (Math|Vector|MakeVector (|((MinX+MaxX)/2) (Variables|Default|GetMin%20X) (Variables|Default|GetMax%20X)) (|((MinY+MaxY)/2) (Variables|Default|GetMin%20Y) (Variables|Default|GetMax%20Y)) 0.0) (Transformation|GetActorLocation))) (Transformation|GetActorForwardVector)) 0.0)
          (Utilities|FlowControl|DoOnce false :!label _label
            (:Completed
              (Transformation|SetActorRotation (Math|Rotator|MakeRotator 0.0 0.0 (.yaw (Math|Random|RandomRotator false)))))))))
    (:then_1
      (Transformation|SetActorLocation (+ (Transformation|GetActorLocation) (* (* DeltaSeconds (Variables|Default|GetSpeed)) (Transformation|GetActorForwardVector))) false false))))

(fn ConstructionScript)

(fn IsActorinBoundaries2D
  (params (Min%20X :type Float%20%28double-precision%29) (Max%20X :type Float%20%28double-precision%29) (Min%20Y :type Float%20%28double-precision%29) (Max%20Y :type Float%20%28double-precision%29))
  (bind _returnvalue (Transformation|GetActorLocation))
  (return (and (Math|Float|InRange(Float) (.x _returnvalue) Min%20X Max%20X) (Math|Float|InRange(Float) (.y _returnvalue) Min%20Y Max%20Y))))