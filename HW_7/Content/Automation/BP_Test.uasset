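; Functional test Blueprint that checks a BP_Movable actor keeps moving within its 2D boundaries.
; On start it takes the first BP_Movable, erroring if none is valid, and derives a timeout from four times the bounds' diagonal travel time at its speed.
; Tick fails the test if the actor leaves bounds or its delayed position check finds it unmoved, and succeeds once the timeout elapses.
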(event `self.ReceivePrepareTest`
  (set `self.TestReady` true))

(event `self.ReceiveStartTest`
  (bind _target (`self.Target`))
  (bind _outactors (`GameplayStatics.GetAllActorsOfClass` "/Game/Blueprints/BP_Movable.BP_Movable_C"))
  (bind _output_get (set `self.Target` (`|GetArrayItem` _outactors)))
  (bind _returnvalue (`self.AssertIsValid` _output_get "BP_Movable found."))
  (if _returnvalue
    (set `self.TimeOut` (* (/ (`KismetMathLibrary.Sqrt` (+ (`KismetMathLibrary.MultiplyMultiply_FloatFloat` (`KismetMathLibrary.Abs` (- (`/Game/Blueprints/BP_Movable.Max X` _target) (`/Game/Blueprints/BP_Movable.Min X` _target))) 2.0) (`KismetMathLibrary.MultiplyMultiply_FloatFloat` (`KismetMathLibrary.Abs` (- (`/Game/Blueprints/BP_Movable.Max Y` _target) (`/Game/Blueprints/BP_Movable.Min Y` _target))) 2.0))) (`KismetMathLibrary.Abs` (`/Game/Blueprints/BP_Movable.Speed` (`self.Target`)))) 4.0))
    (else
      (`self.FinishTest` "Error" "Assertion failed."))))

(event `self.ReceiveTick`
  (params (DeltaSeconds :type "Float (single-precision)"))
  (bind _target (`self.Target`))
  (bind _output_get (set `self.Seconds` (+ DeltaSeconds (`self.Seconds`))))
  (if (< _output_get (`self.TimeOut`))
    (if (`/Game/Blueprints/BP_Movable.Is Actor in Boundaries 2D` _target (`/Game/Blueprints/BP_Movable.Min X` _target) (`/Game/Blueprints/BP_Movable.Max X` _target) (`/Game/Blueprints/BP_Movable.Min Y` _target) (`/Game/Blueprints/BP_Movable.Max Y` _target))
      (`KismetSystemLibrary.Delay` 0.2)
      (if (!= (`self.K2_GetActorLocation` (`self.Target`)) (`self.PreviousPoint`))
        (set `self.PreviousPoint` (`self.K2_GetActorLocation` (`self.Target`)))
        (else
          (`self.FinishTest` "Failed" "Object stuck.")))
      (else
        (`self.FinishTest` "Failed" "Object left boundaries.")))
    (else
      (`self.FinishTest` "Succeeded" "Time out."))))

(fn `IsReady`
  (returns (ReturnValue :type Boolean))
  (return (`self.TestReady`)))

(fn `UserConstructionScript`)