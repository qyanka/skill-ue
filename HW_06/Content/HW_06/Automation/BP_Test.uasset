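; BP_Test is an automated functional test that validates the BP_Exercise actor for the HW_06 assignment.
; It finds the first instance in the level and asserts that its mesh uses GenericHMDMaterial.
; It then spawns a TriggerBox at that actor's transform to provoke an overlap.
; After a short delay, it passes only if the actor is destroyed and a Blueprint_Effect_Explosion exists, otherwise failing with a specific message.
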(event `self.ReceiveStartTest`
  (bind _outactors (`GameplayStatics.GetAllActorsOfClass` "/Game/HW_06/Blueprints/BP_Exercise.BP_Exercise_C"))
  (if (> (`KismetArrayLibrary.Array_Length` _outactors) 0)
    (bind _output_get (set `self.Target` (`|GetArrayItem` _outactors)))
    (bind _returnvalue (`self.AssertEqual_Object` (`PrimitiveComponent.GetMaterial` (`/Game/HW_06/Blueprints/BP_Exercise.StaticMesh` _output_get) 0) "/Engine/VREditor/Devices/Generic/GenericHMDMaterial.GenericHMDMaterial" "Material is set up correctly."))
    (if _returnvalue
      (`|SpawnActorFromClass` "/Script/Engine.TriggerBox" (`self.GetTransform` _output_get) "Undefined" "OverrideRootScale" null null)
      (`KismetSystemLibrary.Delay` 0.2)
      (`/Engine/EditorBlueprintResources/StandardMacros.IsValid` (`self.Target`)
        (:`Is Valid`
          (`self.FinishTest` "Failed" "BP_Exercise is not destroyed!"))
        (:`Is Not Valid`
          (bind _outactors_2 (`GameplayStatics.GetAllActorsOfClass` "/Game/StarterContent/Blueprints/Blueprint_Effect_Explosion.Blueprint_Effect_Explosion_C"))
          (if (> (`KismetArrayLibrary.Array_Length` _outactors_2) 0)
            (`self.FinishTest` "Succeeded" "Congrats!")
            (else
              (`self.FinishTest` "Failed" "Explosion effect is not spawned!")))))
      (else
        (`self.FinishTest` "Failed" "Material setup error!")))
    (else
      (`self.FinishTest` "Failed" "No instances of BP_Exercise found!"))))

(fn `UserConstructionScript`)