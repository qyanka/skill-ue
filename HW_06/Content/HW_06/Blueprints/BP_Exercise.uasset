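; BP_Exercise is a homework exercise actor that reacts to another actor overlapping it.
; On overlap it spawns an actor, with no class shown, at the other actor's transform, then destroys itself if its StaticMesh is valid.
; The construction script applies a material to the mesh's first slot.
; Template comments and unconnected validity checks remain in the event graph.
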(event `self.ReceiveActorBeginOverlap`
  (params (OtherActor :type "Actor Object Reference"))
  ;[1 1 1] Пишите код здесь!
  (`|SpawnActorFromClass` "/Game/StarterContent/Blueprints/Blueprint_Effect_Explosion.Blueprint_Effect_Explosion_C" (`self.GetTransform` OtherActor) "Undefined" "MultiplyWithRoot" null null)
  (`self.StaticMesh`
    (:`then`
      (`self.K2_DestroyActor`))
    (:`else`)))

(fn `UserConstructionScript`
  (`PrimitiveComponent.SetMaterial` (`self.StaticMesh`) 0 (`self.MaterialInterface`)))