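; BP_Actor is an actor that repeatedly teleports its Cube to a random X/Y position and counts the jumps.
; A looping two-second timer started at BeginPlay fires TeleportItem, which prints Counter, moves the Cube and increments Counter.
; The random point is centered on BoundingBox's root world location and also uses that location as the half size, rather than the box's extent.
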(event `self.ReceiveBeginPlay`
  (`KismetSystemLibrary.K2_SetTimerDelegate` (delegate `TeleportItem`) 2.0 true))

(event `TeleportItem`
  (bind _returnvalue (`SceneComponent.K2_GetComponentLocation` (`Actor.RootComponent` (`self.BoundingBox`))))
  (bind (_returnvalue_x _returnvalue_y) (`KismetMathLibrary.BreakVector` (`KismetMathLibrary.RandomPointInBoundingBox` _returnvalue _returnvalue)))
  (`KismetSystemLibrary.PrintString` (`KismetStringLibrary.Conv_IntToString` (`self.counter`)))
  (`SceneComponent.K2_SetWorldLocation` (`self.Cube`) (`KismetMathLibrary.MakeVector` _returnvalue_x _returnvalue_y) false false)
  (bind _result (`/Engine/EditorBlueprintResources/StandardMacros.IncrementInt` (`self.counter`))
    (:`  `
      (set `self.counter` _result))))

(fn `UserConstructionScript`)