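; Functional test for HW_07 that checks the player controller can swap the possessed pawn.
; PrepareTest caches the current player pawn, then StartTest asserts that the GameMode uses BP_HW_07_PlayerController.
; It calls that controller's ExecureChangePawn and passes only if the player pawn differs from the cached one, failing with separate messages for setup and replacement errors.
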(event `self.ReceivePrepareTest`
  (set `self.StartPawn` (`GameplayStatics.GetPlayerPawn` 0))
  (set `self.TestReady` true))

(event `self.ReceiveStartTest`
  (bind _returnvalue (`self.AssertTrue` (== (`GameModeBase.PlayerControllerClass` (`GameplayStatics.GetGameMode`)) "/Game/HW_07/Blueprints/BP_HW_07_PlayerController.BP_HW_07_PlayerController_C") "Desired controller is selected in GameMode."))
  (if _returnvalue
    (bind _asbp_hw_07_player_controller (cast `/Game/HW_07/Blueprints/BP_HW_07_PlayerController` (`GameplayStatics.GetPlayerController` 0)))
    (`/Game/HW_07/Blueprints/BP_HW_07_PlayerController.ExecureChangePawn` _asbp_hw_07_player_controller)
    (bind _returnvalue_2 (`self.AssertFalse` (== (`GameplayStatics.GetPlayerPawn` 0) (`self.StartPawn`)) "Pawn changed on ExecuteChangePawn."))
    (if _returnvalue_2
      (`self.FinishTest` "Succeeded" "Congrats!")
      (else
        (`self.FinishTest` "Failed" "Pawn replacement error!")))
    (else
      (`self.FinishTest` "Failed" "Controller setup error!"))))

(fn `UserConstructionScript`)