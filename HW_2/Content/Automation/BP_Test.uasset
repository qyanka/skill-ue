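; Functional test that checks the damage calculation of the level's first BP_Fighter for expected totals.
; StartTest asserts the fighter exists and seeds its random stream to zero once, making results repeatable across three sequential cases.
; Each case resets SumDamage, calls CalculateDamage with a different enum sequence and fails on a tolerance mismatch.
; StartTest reports success after all cases run, without checking their outcomes.
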(event `self.ReceiveStartTest`
  (bind _outactors (`GameplayStatics.GetAllActorsOfClass` "/Game/Blueprints/BP_Fighter.BP_Fighter_C"))
  (bind _output_get (set `self.fighter` (`|GetArrayItem` _outactors)))
  (bind _returnvalue (`self.AssertIsValid` _output_get "BP_Fighter found."))
  (if _returnvalue
    (`KismetMathLibrary.SetRandomStreamSeed` (`/Game/Blueprints/BP_Fighter.RndStream` (`self.fighter`)))
    (`self.Test1`)
    (`self.Test2`)
    (`self.Test3`)
    (`self.FinishTest` "Succeeded" "Test passed")
    (else
      (`self.FinishTest` "Error" "Assertion failed."))))

(event `Test1`
  (bind _fighter (`self.fighter`))
  (set `/Game/Blueprints/BP_Fighter.SumDamage` 0.0 (`self.fighter`))
  (`/Game/Blueprints/BP_Fighter.CalculateDamage` _fighter "NewEnumerator0")
  (`/Game/Blueprints/BP_Fighter.CalculateDamage` _fighter "NewEnumerator1")
  (`/Game/Blueprints/BP_Fighter.CalculateDamage` _fighter "NewEnumerator1")
  (if (not (`KismetMathLibrary.NearlyEqual_FloatFloat` (`/Game/Blueprints/BP_Fighter.SumDamage` (`self.fighter`)) 11.446901))
    (`self.FinishTest` "Failed" "Test1 failed")))

(event `Test2`
  (bind _fighter (`self.fighter`))
  (set `/Game/Blueprints/BP_Fighter.SumDamage` 0.0 (`self.fighter`))
  (`/Game/Blueprints/BP_Fighter.CalculateDamage` _fighter "NewEnumerator1")
  (`/Game/Blueprints/BP_Fighter.CalculateDamage` _fighter "NewEnumerator2")
  (`/Game/Blueprints/BP_Fighter.CalculateDamage` _fighter "NewEnumerator0")
  (if (not (`KismetMathLibrary.NearlyEqual_FloatFloat` (`/Game/Blueprints/BP_Fighter.SumDamage` (`self.fighter`)) 27.06651))
    (`self.FinishTest` "Failed" "Test2 failed")))

(event `Test3`
  (bind _fighter (`self.fighter`))
  (set `/Game/Blueprints/BP_Fighter.SumDamage` 0.0 (`self.fighter`))
  (`/Game/Blueprints/BP_Fighter.CalculateDamage` _fighter "NewEnumerator2")
  (`/Game/Blueprints/BP_Fighter.CalculateDamage` _fighter "NewEnumerator2")
  (`/Game/Blueprints/BP_Fighter.CalculateDamage` _fighter "NewEnumerator0")
  (if (not (`KismetMathLibrary.NearlyEqual_FloatFloat` (`/Game/Blueprints/BP_Fighter.SumDamage` (`self.fighter`)) 21.2))
    (`self.FinishTest` "Failed" "Test3 failed")))

(fn `UserConstructionScript`)