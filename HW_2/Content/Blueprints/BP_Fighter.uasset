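; BP_Fighter is a fighter Blueprint that accumulates randomized damage for three strike types: Simple, Hook and Kick.
; CalculateDamage switches on the strike, draws values from the RndStream random stream and adds the result to SumDamage.
; Each strike has its own Math Expression formula and random ranges, with Hook and Kick combining two random draws.
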(event Custom|CalculateDamage
  (params (Strike :type E_StrikeTypes%20Enum :default "NewEnumerator0"))
  (bind _rndstream (Variables|Default|GetRndStream))
  (switch Utilities|FlowControl|Switch|SwitchonE_StrikeTypes Strike
    (:NewEnumerator0
      (Variables|Default|SetSumDamage (+ (Variables|Default|GetSumDamage) (|((a*1.200000)+5) (Math|Conversions|ToFloat(Integer) (Math|Random|RandomIntegerinRangefromStream _rndstream 1 4))))))
    (:NewEnumerator1
      (Variables|Default|SetSumDamage (+ (Variables|Default|GetSumDamage) (|(((a*b)+10)/5) (Math|Conversions|ToFloat(Integer) (Math|Random|RandomIntegerinRangefromStream _rndstream 1 7)) (Math|Random|RandomFloatfromStream _rndstream)))))
    (:NewEnumerator2
      (Variables|Default|SetSumDamage (+ (Variables|Default|GetSumDamage) (|((a+10)/b) (Math|Conversions|ToFloat(Integer) (Math|Random|RandomIntegerinRangefromStream _rndstream 4 8)) (Math|Conversions|ToFloat(Integer) (Math|Random|RandomIntegerinRangefromStream _rndstream 1 3))))))))

(event EventBeginPlay)

(event Collision|EventActorBeginOverlap
  (params (OtherActor :type Actor%20Object%20Reference)))

(event EventTick
  (params (DeltaSeconds :type Float%20%28single-precision%29)))

(fn ConstructionScript)